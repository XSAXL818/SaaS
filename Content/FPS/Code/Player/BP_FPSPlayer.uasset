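; First-person player pawn that handles walking and looking through Enhanced Input.
; On BeginPlay it adds the IMC_FPSInput mapping context to its player controller's local player subsystem.
; The move action drives movement along forward and right vectors built from control yaw only, so pitch does not affect direction.
; The look action feeds controller pitch and yaw input.
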(event `self.ReceiveBeginPlay`
  (bind `_as玩家控制器` (cast `PlayerController` (`self.GetController`)))
  (`EnhancedInputSubsystemInterface.AddMappingContext` (pcsubsystem `EnhancedInputLocalPlayerSubsystem` `_as玩家控制器`) "/Game/FPS/Code/Player/System/Input/IMC_FPSInput.IMC_FPSInput" 0 (struct)))

(event `EnhancedInput|/Game/FPS/Code/Player/System/Input/IA_FPS_Move`
  (params (ActionValue :type "Vector2D Structure") (ElapsedSeconds :type "Float (double-precision)") (TriggeredSeconds :type "Float (double-precision)") (InputAction :type "InputAction Object Reference" :default "/Game/FPS/Code/Player/System/Input/IA_FPS_Move.IA_FPS_Move"))
  (bind (_returnvalue_roll _returnvalue_pitch _returnvalue_yaw) (`KismetMathLibrary.BreakRotator` (`self.GetControlRotation`)))
  (:`Triggered`
    (`self.AddMovementInput` (`KismetMathLibrary.GetForwardVector` (`KismetMathLibrary.MakeRotator` 0.0 0.0 _returnvalue_yaw)) ActionValue_X)
    (`self.AddMovementInput` (`KismetMathLibrary.GetRightVector` (`KismetMathLibrary.MakeRotator` 0.0 0.0 _returnvalue_yaw)) ActionValue_Y)))

(event `EnhancedInput|/Game/FPS/Code/Player/System/Input/IA_FPS_Look`
  (params (ActionValue :type "Vector2D Structure") (ElapsedSeconds :type "Float (double-precision)") (TriggeredSeconds :type "Float (double-precision)") (InputAction :type "InputAction Object Reference" :default "/Game/FPS/Code/Player/System/Input/IA_FPS_Look.IA_FPS_Look"))
  (:`Triggered`
    (`self.AddControllerPitchInput` ActionValue_Y)
    (`self.AddControllerYawInput` ActionValue_X)))

(fn `UserConstructionScript`)