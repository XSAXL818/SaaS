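; First-person shooter player character that spawns a VIRTUS weapon on its arms and handles movement, look, aim, fire, reload and death.
; Enhanced Input sets intent flags that Tick resolves into a player state, which drives look sensitivity and, via RepNotify, walk speed.
; Timers smooth aim FOV and delay firing out of sprint.
; Damage drives a health-scaled blood overlay, then retriggerable delays start its fade and timed health regeneration.
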(event `受伤测试`
  (bind _mainui (`self.MainUI`))
  (bind _output_get (set `self.受击画面渲染不透明度` (+ (`self.受击画面渲染不透明度`) 0.2)))
  (`KismetSystemLibrary.PrintString` (`KismetStringLibrary.Conv_DoubleToString` _output_get))
  (`Widget.SetRenderOpacity` (`/Game/FPS/Code/UI/UI_Main.Blood` _mainui) _output_get)
  (`/Game/FPS/Code/UI/UI_Main.BloodFadeAnim` _mainui)
  (`KismetSystemLibrary.Delay` 1.0)
  (`/Game/FPS/Code/UI/UI_Main.StopBloodFadeAnim` _mainui))

(event `self.ReceiveBeginPlay`
  (bind `_as玩家控制器` (cast `PlayerController` (`self.GetController`)))
  (`EnhancedInputSubsystemInterface.AddMappingContext` (pcsubsystem `EnhancedInputLocalPlayerSubsystem` `_as玩家控制器`) "/Game/FPS/Code/Player/System/Input/IMC_FPSInput.IMC_FPSInput" 0 (struct))
  (`self.SpawnWeapon` "/Game/FPS/Code/Weapon/BP_VIRTUS.BP_VIRTUS_C")
  (`CameraComponent.SetFieldOfView` (`self.Camera`) (`self.DefaultFOV`))
  (bind _returnvalue (`|CreateWidget` "/Game/FPS/Code/UI/UI_Main.UI_Main_C"))
  (bind _output_get (set `self.MainUI` _returnvalue))
  (`UserWidget.AddToViewport` _output_get 0))

(event `self.ReceiveTick`
  (params (DeltaSeconds :type "Float (single-precision)"))
  (`self.UpdatePlayerState`)
  (`KismetSystemLibrary.PrintString` (`|GetEnumeratorNameAsString` (`self.E_PlayerState`)) true true (struct :`G` 0.66 :`B` 1.0 :`A` 1.0) 0.0)
  (`KismetSystemLibrary.PrintString` (`|GetEnumeratorNameAsString` (`self.E_AimState`)) true true (struct :`R` 1.0 :`G` 0.55405 :`B` 0.717507 :`A` 1.0) 0.0)
  (`KismetSystemLibrary.PrintString` (`KismetStringLibrary.Concat_StrStr` "blood渲染不透明度：" (`KismetStringLibrary.Conv_DoubleToString` (`Widget.RenderOpacity` (`/Game/FPS/Code/UI/UI_Main.Blood` (`self.MainUI`))))) true true (struct :`R` 1.0 :`G` 0.140276 :`B` 0.987664 :`A` 1.0) 0.0)
  (`KismetSystemLibrary.PrintString` (`KismetStringLibrary.Concat_StrStr` "玩家血量：" (`KismetStringLibrary.Conv_DoubleToString` (`self.Health`))) true true (struct :`R` 0.5 :`B` 0.011531 :`A` 1.0) 0.0))

(event `self.ReceiveAnyDamage`
  (params (Damage :type "Float (single-precision)") (DamageType :type "DamageType Object Reference") (InstigatedBy :type "Controller Object Reference") (DamageCauser :type "Actor Object Reference"))
  (bind _mainui (`self.MainUI`))
  (`KismetSystemLibrary.K2_ClearAndInvalidateTimerHandle` (`self.HealHeathHandle`))
  (bind _output_get (set `self.Health` (- (`self.Health`) Damage)))
  (if (<= _output_get 0.0)
    (`|ExecutionSequence`
      (:`then_0`
        (`/Game/FPS/Code/UI/UI_Main.StopBloodFadeAnim` (`self.MainUI`))
        (set `Widget.RenderOpacity` 1.0 (`/Game/FPS/Code/UI/UI_Main.Blood` (`self.MainUI`)))
        (set `self.IsDead` true)
        (`self.DisableInput` (`GameplayStatics.GetPlayerController` 0))))
    (else
      (`|ExecutionSequence`
        (:`then_0`
          (`/Game/FPS/Code/UI/UI_Main.StopBloodFadeAnim` _mainui)
          (`self.UpdateOpacityWithHealth`)
          (`KismetSystemLibrary.Delay` 0.1)
          (`Widget.SetRenderOpacity` (`/Game/FPS/Code/UI/UI_Main.Blood` _mainui) (`self.受击画面渲染不透明度`))
          (`KismetSystemLibrary.RetriggerableDelay` 2.0)
          (if (not (`self.IsDead`))
            (`/Game/FPS/Code/UI/UI_Main.BloodFadeAnim` _mainui)))
        (:`then_1`
          (`KismetSystemLibrary.RetriggerableDelay` 5.0)
          (bind _returnvalue (`KismetSystemLibrary.K2_SetTimerDelegate` (delegate `HealHealth`) 0.1 true))
          (set `self.HealHeathHandle` _returnvalue))))))

(event `HealHealth`
  (if (`self.IsDead`)
    (`KismetSystemLibrary.K2_ClearAndInvalidateTimerHandle` (`self.HealHeathHandle`))
    (else
      (bind _output_get (set `self.Health` (`KismetMathLibrary.FClamp` (+ (`self.Health`) 1.0) 0.0 (`self.MaxHealth`))))
      (if (>= _output_get (`self.MaxHealth`))
        (`KismetSystemLibrary.K2_ClearAndInvalidateTimerHandle` (`self.HealHeathHandle`))))))

(event `EnhancedInput|/Game/FPS/Code/Player/System/Input/IA_FPS_Move`
  (params (ActionValue :type "Vector2D Structure") (ElapsedSeconds :type "Float (double-precision)") (TriggeredSeconds :type "Float (double-precision)") (InputAction :type "InputAction Object Reference" :default "/Game/FPS/Code/Player/System/Input/IA_FPS_Move.IA_FPS_Move"))
  (bind (_returnvalue_roll _returnvalue_pitch _returnvalue_yaw) (`KismetMathLibrary.BreakRotator` (`self.GetControlRotation`)))
  ; 摄像机或者说准心的旋转,第一人称游戏直接用actor的也没啥问题，但第三人称就有问题了
  (:`Triggered`
    (bind _output_get (set `self.Move X` ActionValue_X))
    (bind _output_get_2 (set `self.Move Y` ActionValue_Y))
    (`self.AddMovementInput` (`KismetMathLibrary.GetForwardVector` (`KismetMathLibrary.MakeRotator` 0.0 0.0 _returnvalue_yaw)) _output_get)
    (`self.AddMovementInput` (`KismetMathLibrary.GetRightVector` (`KismetMathLibrary.MakeRotator` 0.0 0.0 _returnvalue_yaw)) _output_get_2)
    (if (not (> (`self.Move X`) 0.0))
      (set `self.Want To Run` false)))
  (:`Completed`
    (set `self.Move X` 0.0)
    (set `self.Move Y` 0.0)
    (set `self.Want To Run` false)))

(event `EnhancedInput|/Game/FPS/Code/Player/System/Input/IA_FPS_Look`
  (params (ActionValue :type "Vector2D Structure") (ElapsedSeconds :type "Float (double-precision)") (TriggeredSeconds :type "Float (double-precision)") (InputAction :type "InputAction Object Reference" :default "/Game/FPS/Code/Player/System/Input/IA_FPS_Look.IA_FPS_Look"))
  (:`Triggered`
    (`self.AddControllerPitchInput` (* (`self.MouseSensitivity`) (`self.UpdateScopeSensitivity`) ActionValue_Y))
    (`self.AddControllerYawInput` (* ActionValue_X (`self.MouseSensitivity`) (`self.UpdateScopeSensitivity`)))))

(event `EnhancedInput|/Game/FPS/Code/Player/System/Input/IA_FPS_Run`
  (params (ActionValue :type Boolean) (ElapsedSeconds :type "Float (double-precision)") (TriggeredSeconds :type "Float (double-precision)") (InputAction :type "InputAction Object Reference" :default "/Game/FPS/Code/Player/System/Input/IA_FPS_Run.IA_FPS_Run"))
  (:`Started`
    (`self.CancelRunToWalk`)
    (`KismetSystemLibrary.K2_ClearAndInvalidateTimerHandle` (`self.RunToWalkTimerHandle`))
    (if (`|EnumEquality` (`self.E_PlayerState`) "NewEnumerator3")
      (if (< (- (`KismetSystemLibrary.GetGameTimeInSeconds`) (`self.LastRunTime`)) 0.25)
        (set `self.Want To Run` true)
        (set `self.Want To Aim` false)
        (`self.UpdateFOV` false)
        (else
          (set `self.LastRunTime` (`KismetSystemLibrary.GetGameTimeInSeconds`))))
      (else
        (bind _output_get (set `self.Want To Run` (not (`self.Want To Run`))))
        (set `self.Want To Aim` false)
        (if (not _output_get)
          (set `self.IsInRunToWalk` true)
          (bind _returnvalue (`KismetSystemLibrary.K2_SetTimerDelegate` (delegate `CancelRunToWalk`) 0.3))
          (set `self.RunToWalkTimerHandle` _returnvalue))))))

(event `EnhancedInput|/Game/FPS/Code/Player/System/Input/IA_FPS_Aim`
  (params (ActionValue :type Boolean) (ElapsedSeconds :type "Float (double-precision)") (TriggeredSeconds :type "Float (double-precision)") (InputAction :type "InputAction Object Reference" :default "/Game/FPS/Code/Player/System/Input/IA_FPS_Aim.IA_FPS_Aim"))
  (:`Started`
    (switch `/Game/FPS/Code/Player/System/Enum/E_WeaponState` (`/Game/FPS/Code/Weapon/Base/BP_FPS_WeaponBase.WeaponState` (`self.CurrentWeapon`))
      (:`NewEnumerator0`
        _)
      (:`NewEnumerator1`
        _))
    (bind _output_get (set `self.Want To Aim` (not (`self.Want To Aim`))))
    (if _output_get
      (`self.UpdateFOV` true)
      (else
        (`self.UpdateFOV` false)))))

(event `CancelRunToWalk`
  (set `self.IsInRunToWalk` false))

(event `UpdateFOV`
  (params (`bTo Aim` :type Boolean))
  (`KismetSystemLibrary.K2_ClearAndInvalidateTimerHandle` (`self.UpdateFOVTimer`))
  (bind _returnvalue (`KismetSystemLibrary.K2_SetTimerDelegate` (delegate `UpdateFOV Per Frame`) (`GameplayStatics.GetWorldDeltaSeconds`) true true))
  (set `self.UpdateFOVTimer` _returnvalue))

(event `UpdateFOV Per Frame`
  (if (stale `UpdateFOV` `bTo Aim`)
    (set `self.TargetFOV` (`self.AimFOV`))
    (else
      (set `self.TargetFOV` (`self.DefaultFOV`))))
  (bind _returnvalue (`KismetMathLibrary.FInterpTo` (`CameraComponent.FieldOfView` (`self.Camera`)) (`self.TargetFOV`) (`GameplayStatics.GetWorldDeltaSeconds`) 8.0))
  (`CameraComponent.SetFieldOfView` (`self.Camera`) _returnvalue)
  (if (`KismetMathLibrary.NearlyEqual_FloatFloat` _returnvalue (`self.TargetFOV`) 1.0)
    (`KismetSystemLibrary.K2_ClearAndInvalidateTimerHandle` (`self.UpdateFOVTimer`))))

(event `ResetFire`
  (goto _label :!via `Reset`))

(event `EnhancedInput|/Game/FPS/Code/Player/System/Input/IA_FPS_Fire`
  (params (ActionValue :type Boolean) (ElapsedSeconds :type "Float (double-precision)") (TriggeredSeconds :type "Float (double-precision)") (InputAction :type "InputAction Object Reference" :default "/Game/FPS/Code/Player/System/Input/IA_FPS_Fire.IA_FPS_Fire"))
  (:`Triggered`
    (`/Engine/EditorBlueprintResources/StandardMacros.DoOnce` false :!label _label
      (:`Completed`
        (if (`self.IsInRunToWalk`)
          (`self.ResetFire`)
          (else
            (set `self.Want To Fire` true)
            (if (`self.IsDead`)
              _
              (elif (`self.IsFiring`)
                _
                (elif (`|EnumInequality` (`self.E_PlayerState`) "NewEnumerator2")
                  (message `/Game/FPS/Code/BlueprintInterface/BI_Fire.StartWeaponFire` (`self.CurrentWeapon`))
                  (else
                    (`KismetSystemLibrary.Delay` 0.3)
                    (if (`self.Want To Fire`)
                      (set `self.IsFiring` true)
                      (message `/Game/FPS/Code/BlueprintInterface/BI_Fire.StartWeaponFire` (`self.CurrentWeapon`))))))))))))
  (:`Completed`
    (`/Game/FPS/Code/Weapon/Base/BP_FPS_WeaponBase.StopWeaponFire` (`self.CurrentWeapon`))
    (set `self.IsFiring` false)
    (set `self.Want To Fire` false)
    (`self.ResetFire`)))

(event `EnhancedInput|/Game/FPS/Code/Player/System/Input/IA_FPS_Reload`
  (params (ActionValue :type Boolean) (ElapsedSeconds :type "Float (double-precision)") (TriggeredSeconds :type "Float (double-precision)") (InputAction :type "InputAction Object Reference" :default "/Game/FPS/Code/Player/System/Input/IA_FPS_Reload.IA_FPS_Reload"))
  (:`Started`
    (`/Game/FPS/Code/Weapon/Base/BP_FPS_WeaponBase.StartReload` (`self.CurrentWeapon`))))

(fn `CancelAim`
  (if (`self.Want To Aim`)
    (set `self.Want To Aim` false)
    (`self.UpdateFOV` false)))

(fn `OnRep_E_PlayerState`
  (`self.UpdateMoveSpeed`))

(fn `SpawnWeapon`
  (params (WeaponClass :type "/Game/FPS/Code/Weapon/BP_VIRTUS Class Reference"))
  (bind _returnvalue (`|SpawnActorFromClass` WeaponClass (`KismetMathLibrary.MakeTransform` (0.0 0.0 0.0)) "Undefined" "MultiplyWithRoot" self null))
  (bind _asbp_fps_weapon_base (cast `/Game/FPS/Code/Weapon/Base/BP_FPS_WeaponBase` _returnvalue))
  (bind _output_get (set `self.CurrentWeapon` _asbp_fps_weapon_base))
  (bind _aim_socket_location (`/Game/FPS/Code/Weapon/Base/BP_FPS_WeaponBase.GetAimSocketLocation` _output_get))
  (set `self.Aim Socket Location` _aim_socket_location)
  (`self.K2_AttachToComponent` _output_get (`self.Arm`) "None" "KeepRelative" "KeepRelative" "KeepRelative" true)
  (return))

(fn `UpdateMoveSpeed`
  (set `CharacterMovementComponent.MaxWalkSpeed` (select `/Game/FPS/Code/Player/System/Enum/E_FPS_PlayerState` (`self.E_PlayerState`) :`NewEnumerator0` 400.0 :`NewEnumerator1` 400.0 :`NewEnumerator2` 600.0 :`NewEnumerator3` 265.0 :!type "Float (single-precision)") (`self.CharacterMovement`)))

(fn `UpdateOpacityWithHealth`
  (set `self.受击画面渲染不透明度` (- 1.0 (/ (`self.Health`) 100.0))))

(fn `UpdatePlayerState`
  ; 目前有个小bug，walk和idel的判断根据角色移动速度，如果角色站在移动平台，会被判断为walk，但当前不会出现此类功能
  (if (`self.Want To Aim`)
    (set `self.E_PlayerState` "NewEnumerator3")
    (bind _aim_socket_location (`/Game/FPS/Code/Weapon/Base/BP_FPS_WeaponBase.GetAimSocketLocation` (`self.CurrentWeapon`)))
    (set `self.Aim Socket Location` _aim_socket_location)
    (if (< (`KismetMathLibrary.VSize` (`MovementComponent.Velocity` (`self.CharacterMovement`))) 10.0)
      (set `self.E_AimState` "NewEnumerator4")
      (else
        (set `self.E_AimState` "NewEnumerator5")))
    (elif (> (`self.Move X`) 0.0)
      (if (`self.Want To Run`)
        (if (`self.Want To Fire`)
          (set `self.E_PlayerState` "NewEnumerator1")
          (else
            (set `self.E_PlayerState` "NewEnumerator2")))
        (else
          (set `self.E_PlayerState` "NewEnumerator1")))
      (elif (> (`KismetMathLibrary.VSize` (`MovementComponent.Velocity` (`self.CharacterMovement`))) 0.0)
        (set `self.E_PlayerState` "NewEnumerator1")
        (else
          (set `self.E_PlayerState` "NewEnumerator0"))))))

(fn `UpdateScopeSensitivity`
  (returns (OutSensitivity :type "Float (double-precision)"))
  (return (select `/Game/FPS/Code/Player/System/Enum/E_FPS_PlayerState` (`self.E_PlayerState`) :`NewEnumerator0` 1.0 :`NewEnumerator1` 1.0 :`NewEnumerator2` 1.0 :`NewEnumerator3` 0.5)))

(fn `UserConstructionScript`)