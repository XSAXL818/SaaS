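; BP_PhysCube is a cube actor with a configurable physical material, text label and color, apparently for showcasing physical materials.
; The construction script applies the material override to the cube, sets the TextRender text, and writes the "Color" parameter on the cube's materials through a duplicated call.
; BeginPlay reapplies the physical material and text, but not the color.
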(event `self.ReceiveBeginPlay`
  (`PrimitiveComponent.SetPhysMaterialOverride` (`self.Cube`) (`self.Phys Material`))
  (`TextRenderComponent.K2_SetText` (`self.TextRender`) (`self.Text`)))

(fn `UserConstructionScript`
  (`PrimitiveComponent.SetPhysMaterialOverride` (`self.Cube`) (`self.Phys Material`))
  (`TextRenderComponent.K2_SetText` (`self.TextRender`) (`self.Text`))
  (`MeshComponent.SetColorParameterValueOnMaterials` (`self.Cube`) "Color" (`self.Parameter Value`))
  (`MeshComponent.SetColorParameterValueOnMaterials` (`self.Cube`) "Color" (`self.Parameter Value`)))