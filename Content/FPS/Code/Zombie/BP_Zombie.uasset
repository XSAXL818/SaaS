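; Zombie character Blueprint that handles health, hit reactions by body part and death.
; AnyDamage subtracts health and, on non-lethal hits, reads the surface type from a DT_Zombie damage type.
; Body hits briefly slow movement, the first leg hit slows it permanently, and hand hits clear Attackable.
; Death unpossesses it, ragdolls the mesh and destroys it after a delay; Tick prints walk speed for debugging.
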(event `self.ReceiveTick`
  (params (DeltaSeconds :type "Float (single-precision)"))
  (`KismetSystemLibrary.PrintString` (`KismetStringLibrary.Conv_DoubleToString` (`CharacterMovementComponent.MaxWalkSpeed` (`self.CharacterMovement`))) true true (struct :`G` 0.66 :`B` 1.0 :`A` 1.0) 0.0))

(event `self.ReceiveAnyDamage`
  (params (Damage :type "Float (single-precision)") (DamageType :type "DamageType Object Reference") (InstigatedBy :type "Controller Object Reference") (DamageCauser :type "Actor Object Reference"))
  (bind _charactermovement (`self.CharacterMovement`))
  (bind _charactermovement_2 (`self.CharacterMovement`))
  (bind _mesh (`self.Mesh`))
  (bind _charactermovement_3 (`self.CharacterMovement`))
  (bind _output_get (set `self.Health` (- (`self.Health`) Damage)))
  (if (<= _output_get 0.0)
    (`/Engine/EditorBlueprintResources/StandardMacros.DoOnce` false
      (:`Completed`
        (set `self.bDead` true)
        (`Controller.UnPossess` (`self.GetController`))
        (`PrimitiveComponent.SetCollisionEnabled` (`self.CapsuleComponent`) "NoCollision")
        (set `SkeletalMeshComponent.bPauseAnims` (`self.bDead`) _mesh)
        (`PrimitiveComponent.SetCollisionProfileName` _mesh "Ragdoll" true)
        (`PrimitiveComponent.SetSimulatePhysics` _mesh true)
        (`KismetSystemLibrary.Delay` 3.0)
        (`self.K2_DestroyActor`)))
    (else
      (bind _asdt_zombie (cast `/Game/FPS/Code/DamgaeTpye/DT_Zombie` DamageType))
      (switch `EPhysicalSurface` (`/Game/FPS/Code/DamgaeTpye/DT_Zombie.PhysicalSurface` _asdt_zombie)
        (:`SurfaceType4`
          (`/Engine/EditorBlueprintResources/StandardMacros.DoOnce` false :!label _label
            (:`Completed`
              (set `CharacterMovementComponent.MaxWalkSpeed` (- (`CharacterMovementComponent.MaxWalkSpeed` _charactermovement_2) 25.0) _charactermovement_2)
              (`KismetSystemLibrary.Delay` 0.2)
              (set `CharacterMovementComponent.MaxWalkSpeed` (+ (`CharacterMovementComponent.MaxWalkSpeed` _charactermovement_3) 25.0) _charactermovement_3)
              (goto _label :!via `Reset`))))
        (:`SurfaceType9`
          (`/Engine/EditorBlueprintResources/StandardMacros.DoOnce` false
            (:`Completed`
              (set `CharacterMovementComponent.MaxWalkSpeed` (- (`CharacterMovementComponent.MaxWalkSpeed` _charactermovement) 100.0) _charactermovement))))
        (:`SurfaceType10`
          (set `self.bAttackable` false))))))

(fn `UserConstructionScript`)