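; Base weapon Blueprint for FPS guns, handling automatic fire feedback and exposing the aim socket location.
; StartWeaponFire caches the player, checks ammo once, then fires immediately and on a looping FireRate timer until StopWeaponFire clears it.
; Each shot plays state-selected weapon and arm montages (none for Run), sound, muzzle flash and a randomly rotated casing.
; No ammo decrement or hit logic is present here.
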(event `FireIntermal`
  (bind _returnvalue (`SceneComponent.GetSocketTransform` (`self.Weapon`) "Casing" "RTS_World"))
  (`|PlayMontage` (`self.Weapon`) (select `/Game/FPS/Code/Player/System/Enum/E_FPS_PlayerState` (`/Game/FPS/Code/Player/BP_FPS_Player.E_PlayerState` (`self.FPSPlayer`)) :`NewEnumerator0` (`self.WeaponIdleFireMontage`) :`NewEnumerator1` (`self.WeaponWalkFireMontage`) :`NewEnumerator3` (`self.WeaponAimFireMontage`))
    (:`then`
      (`|PlayMontage` (`/Game/FPS/Code/Player/BP_FPS_Player.Arm` (`self.FPSPlayer`)) (select `/Game/FPS/Code/Player/System/Enum/E_FPS_PlayerState` (`/Game/FPS/Code/Player/BP_FPS_Player.E_PlayerState` (`self.FPSPlayer`)) :`NewEnumerator0` (`self.PlayerIdleFireMontage`) :`NewEnumerator1` (`self.PlayerWalkFireMontage`) :`NewEnumerator3` (`self.PlayerAimFireMontage`))
        (:`then`
          (`GameplayStatics.PlaySound2D` "/Game/FPS/Code/Weapon/MetaSound/MS_VIRTUS.MS_VIRTUS" 1.0 1.0 0.0 null null)
          (`NiagaraFunctionLibrary.SpawnSystemAttached` "/Game/FPSAssets/ShotSystem/Shot_VFX/VIRTUS_MuzzleFlash.VIRTUS_MuzzleFlash" (`self.Barrel`) "Muzzle" (0.0 0.0 0.0) (struct) "KeepRelativeOffset" true)
          (`|SpawnActorFromClass` "/Game/FPS/Code/Weapon/BP_Casing.BP_Casing_C" (`KismetMathLibrary.MakeTransform` (.location _returnvalue) (`KismetMathLibrary.MakeRotator` (+ (.roll (.rotation _returnvalue)) (`KismetMathLibrary.RandomFloatInRange` -35.0 35.0)) (+ (.pitch (.rotation _returnvalue)) (`KismetMathLibrary.RandomFloatInRange` -35.0 35.0)) (+ (.yaw (.rotation _returnvalue)) (`KismetMathLibrary.RandomFloatInRange` -15.0 15.0)))) "Undefined" "MultiplyWithRoot" null null))))))

(event `/Game/FPS/Code/BlueprintInterface/BI_Fire.StartWeaponFire`
  (params (FPSPlayer :type "/Game/FPS/Code/Player/BP_FPS_Player Object Reference"))
  (set `self.FPSPlayer` FPSPlayer)
  (if (> (`self.CurrentAmmo`) 0)
    (`self.FireIntermal`)
    (bind _returnvalue (`KismetSystemLibrary.K2_SetTimerDelegate` (delegate `FireIntermal`) (`self.FireRate`) true))
    (set `self.WeaponFireTimerHandle` _returnvalue)))

(event `StopWeaponFire`
  (`KismetSystemLibrary.K2_ClearAndInvalidateTimerHandle` (`self.WeaponFireTimerHandle`)))

(fn `GetAimSocketLocation`
  (returns (`Aim Socket Location` :type "Vector Structure"))
  (return (`SceneComponent.GetSocketLocation` (`self.Weapon`) "AimSocket")))

(fn `UserConstructionScript`)