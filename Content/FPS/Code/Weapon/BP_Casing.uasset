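; BP_Casing is an ejected bullet casing actor for the FPS weapon system.
; On spawn it randomizes its projectile launch speed and tumbling rotation rate.
; The first bounce stops the spin and plays an impact sound once.
; When projectile movement stops, the casing mesh switches to physics simulation with a small downward velocity so it settles naturally.
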(event `self.ReceiveBeginPlay`
  (bind _returnvalue (`KismetMathLibrary.RandomFloatInRange` -1800.0 1800.0))
  (set `ProjectileMovementComponent.InitialSpeed` (`KismetMathLibrary.RandomFloatInRange` 450.0 500.0) (`self.ProjectileMovement`))
  (set `RotatingMovementComponent.RotationRate` (`KismetMathLibrary.MakeRotator` _returnvalue _returnvalue _returnvalue) (`self.RotatingMovement`)))

(event `self.ProjectileMovement.OnProjectileBounce`
  (params (ImpactResult :type "HitResult Structure (by ref)") (ImpactVelocity :type "Vector Structure (by ref)"))
  (`/Engine/EditorBlueprintResources/StandardMacros.DoOnce` false
    (:`Completed`
      (`ActorComponent.Deactivate` (`self.RotatingMovement`))
      (`GameplayStatics.SpawnSoundAtLocation` "/Game/FPSAssets/XL_FPSPack/Weapons/Common/Sounds/Shell_Impact/Bullet_Impact.Bullet_Impact" (`self.K2_GetActorLocation`) (struct) 0.5 1.0 0.0 null null))))

(event `self.ProjectileMovement.OnProjectileStop`
  (params (ImpactResult :type "HitResult Structure (by ref)"))
  (bind _casing (`self.Casing`))
  (`PrimitiveComponent.SetSimulatePhysics` _casing true)
  (`PrimitiveComponent.SetPhysicsLinearVelocity` _casing (0.0 0.0 -50.0) false "None"))

(fn `UserConstructionScript`)