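; Automatic swinging door actor that opens when a BP_MyCharacter enters its Box trigger and closes when it leaves.
; On overlap, GetDirection dots the character-to-door vector with the Arrow's forward vector to pick the swing sign from the approach side.
; A Timeline lerps the door's world yaw from its BeginPlay value to that signed OpenAngle offset, reversing on exit.
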(event `self.ReceiveBeginPlay`
  (bind (_returnvalue_roll _returnvalue_pitch _returnvalue_yaw) (`KismetMathLibrary.BreakRotator` (`SceneComponent.K2_GetComponentRotation` (`self.Door`))))
  (set `self.InitialYaw` _returnvalue_yaw))

(event `self.ReceiveTick`
  (params (DeltaSeconds :type "Float (single-precision)")))

(event `self.Box.OnComponentBeginOverlap`
  (params (OverlappedComponent :type "PrimitiveComponent Object Reference") (OtherActor :type "Actor Object Reference") (OtherComp :type "PrimitiveComponent Object Reference") (OtherBodyIndex :type Integer) (bFromSweep :type Boolean) (SweepResult :type "HitResult Structure (by ref)"))
  (bind _door (`self.Door`))
  (bind (_returnvalue_roll _returnvalue_pitch) (`KismetMathLibrary.BreakRotator` (`SceneComponent.K2_GetComponentRotation` _door)))
  (bind _asbp_my_character (cast `/Game/Code/BP_MyCharacter` OtherActor))
  (bind _direction (`self.GetDirection` (`SceneComponent.K2_GetComponentLocation` (`self.Door`)) (`SceneComponent.K2_GetComponentLocation` (`Character.Mesh` _asbp_my_character)) (`SceneComponent.GetForwardVector` (`self.Arrow`))))
  (set `self.OpenDirection` _direction)
  (set `self.TargetAngle` (+ (* (`self.OpenAngle`) (`self.OpenDirection`)) (`self.InitialYaw`)))
  (bind (_direction_2 `_新建轨道_0`) (`Timeline|时间轴` :!label _label)
    (:`Update`
      (`SceneComponent.K2_SetWorldRotation` _door (`KismetMathLibrary.MakeRotator` _returnvalue_roll _returnvalue_pitch (`KismetMathLibrary.Lerp` (`self.InitialYaw`) (`self.TargetAngle`) `_新建轨道_0`)) false false))))

(event `self.Box.OnComponentEndOverlap`
  (params (OverlappedComponent :type "PrimitiveComponent Object Reference") (OtherActor :type "Actor Object Reference") (OtherComp :type "PrimitiveComponent Object Reference") (OtherBodyIndex :type Integer))
  (cast `/Game/Code/BP_MyCharacter` OtherActor)
  (goto _label :!via `Reverse`))

(fn `GetDirection`
  (params (DoorLocation :type "Vector Structure") (ActorLocation :type "Vector Structure") (DoorForward :type "Vector Structure"))
  (returns (Direction :type "Float (double-precision)"))
  (if (>= (`KismetMathLibrary.Dot_VectorVector` (- DoorLocation ActorLocation) DoorForward) 0.0)
    (return 1.0)
    (else
      (return -1.0))))

(fn `UserConstructionScript`)